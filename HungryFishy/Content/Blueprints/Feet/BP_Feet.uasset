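; BP_Feet is a rigged feet Blueprint that reacts to a Tickle event with sound and animation.
; Its construction script initializes the Control Rig component from Rigged_Feet's bone transforms, and the pre-initialize delegate maps the skeletal mesh to the rig.
; Tickle plays the MS_Lynx sound, then creates and plays a sped-up LS_Feet level sequence, with its loop count set by NumberOfLoopFeet.
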(event OnPreInitializeDelegate(ControlRig)
  (params (Component :type Control%20Rig%20Component%20Object%20Reference))
  (Class|ControlRigComponent|AddMappedCompleteSkeletalMesh Component (Variables|Default|GetSkeletalMesh)))

(event Custom|Tickle
  (Audio|PlaySoundatLocation "/Game/Audio/SFX/MS_Lynx.MS_Lynx" "0, 0, 0" "0, 0, 0" 1.0 1.0 0.0 0 0 0 0)
  (bind _outactor (Sequencer|Player|CreateLevelSequencePlayer "/Game/Blueprints/Feet/LS_Feet.LS_Feet" (Utilities|Struct|MakeMovieSceneSequencePlaybackSettings false (Utilities|Struct|MakeMovieSceneSequenceLoopCount (Variables|Default|GetNumberOfLoopFeet)) 1.5 0.0 false false false false false false false false)))
  (Sequencer|Player|Play (Variables|/Script/LevelSequence.LevelSequenceActor|GetSequencePlayer _outactor) :!class /Script/MovieScene.MovieSceneSequencePlayer))

(fn ConstructionScript
  (bind _controlrig (Variables|Default|GetControlRig))
  (Initialization|Initialize _controlrig)
  (Class|ControlRigComponent|SetBoneInitialTransformsfromSkeletalMesh _controlrig "/Game/Meshes/Feet/Rigged_Feet.Rigged_Feet"))