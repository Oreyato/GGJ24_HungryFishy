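; Food spawner that periodically drops random batches of food actors just below its spawn point, driven by wave definitions in WavesData.
; Timed waves advance up to the last index, each setting a random duration, drop quantity and spawn period ranges, and per-food drop chances.
; Self-rescheduling spawn timers pick each food by cumulative-probability roll.
; SetWave restarts the wave timer from a given index; SpawnFood_OLD is an older random-scale spawn variant.
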(event Custom|SpawnFood_OLD
  (bind _spawn_point (Variables|Default|GetSpawn%20Point))
  (bind _returnvalue (Transformation|GetWorldTransform _spawn_point))
  (Variables|OLD|SetUniformRandomScale (Math|Random|RandomFloatinRange 0.4 0.6))
  (Game|SpawnActorfromClass (.OutItem (Utilities|Array|Random (Variables|OLD|GetFood))) (Math|Transform|MakeTransform (.location _returnvalue) (.rotation _returnvalue) (* "1.000000,1.000000,1.000000" (Variables|OLD|GetUniformRandomScale))) "Undefined" "MultiplyWithRoot" 0 0))

(event Custom|AutoWaveChange
  (CallFunction|NextWave)
  (bind _returnvalue (Utilities|Time|SetTimerbyEvent (EventDispatchers|CreateEvent :!event Custom|AutoWaveChange) (Variables|Default|GetCurrentWaveDuration)))
  (Variables|Default|SetAutoWaveChangeTH _returnvalue))

(event Custom|SpawnFood
  (bind _current_wave (Variables|Default|GetCurrent%20Wave))
  (bind _current_wave_2 (Variables|Default|GetCurrent%20Wave))
  (Variables|Default|SetSpawnQuantity (Math|Random|RandomIntegerinRange (Variables|/Game/Blueprints/Spawners/Waves/PDA_SpawningWave.PDA_SpawningWave_C|GetMinDropQuantity _current_wave_2) (Variables|/Game/Blueprints/Spawners/Waves/PDA_SpawningWave.PDA_SpawningWave_C|GetMaxDropQuantity _current_wave_2)))
  (for _index (range 0 (Variables|Default|GetSpawnQuantity))
    ;[1 1 1] Spawn random food
    (bind _food (CallFunction|GetRandomFood))
    (Game|SpawnActorfromClass (Variables|/Game/Blueprints/Food/Data/PDA_Food.PDA_Food_C|GetClass _food) (Math|Transform|MakeTransform (- (.location (Transformation|GetWorldTransform (Variables|Default|GetSpawn%20Point))) "0.000000,0.000000,50.000000") "0, 0, 0" "1.000000,1.000000,1.000000") "AdjustIfPossibleButAlwaysSpawn" "MultiplyWithRoot" 0 0))
  (bind _output_get (Variables|Default|SetSpawnPeriod (Math|Random|RandomFloatinRange (Variables|/Game/Blueprints/Spawners/Waves/PDA_SpawningWave.PDA_SpawningWave_C|GetMinSpawnPeriod _current_wave) (Variables|/Game/Blueprints/Spawners/Waves/PDA_SpawningWave.PDA_SpawningWave_C|GetMaxSpawnPeriod _current_wave))))
  (bind _returnvalue (Utilities|Time|SetTimerbyEvent (EventDispatchers|CreateEvent :!event Custom|SpawnFood) _output_get))
  (Variables|Default|SetSpawnFoodTH _returnvalue))

(event EventBeginPlay
  ;[1 0.8942 0.1979] Comment
  ;;[1 1 1] Get max wave index
  (Variables|Default|SetMaxWaveIndex (- (Utilities|Array|Length (Variables|/Game/Blueprints/Spawners/PDA_WavesMain.PDA_WavesMain_C|GetWaves (Variables|Default|GetWavesData))) 1))
  (CallFunction|AutoWaveChange))

(fn ConstructionScript)

(fn NextWave
  ;[1 1 1] Reset auto wave change
  (Utilities|Time|ClearandInvalidateTimerbyHandle (Variables|Default|GetAutoWaveChangeTH))
  ;[1 1 1] Stop NewSpawnTry
  (Utilities|Time|ClearandInvalidateTimerbyHandle (Variables|Default|GetSpawnFoodTH))
  ;[1 1 1] Make sure (current wave index + 1) is <= max wave index
  (bind _result (Math|Integer|IncrementInt (Variables|Default|GetCurrentWaveIndex))
    (:%20%20
      (Variables|Default|SetCurrentWaveIndex (Math|Integer|Clamp(Integer) _result 0 (Variables|Default|GetMaxWaveIndex)))
      ;[1 1 1] Retrieve current wave
      (Variables|Default|SetCurrent%20Wave (Utilities|Array|Get(acopy) (Variables|/Game/Blueprints/Spawners/PDA_WavesMain.PDA_WavesMain_C|GetWaves (Variables|Default|GetWavesData)) (Variables|Default|GetCurrentWaveIndex)))
      ;[1 1 1] Set wave duration
      (Variables|Default|SetCurrentWaveDuration (Math|Random|RandomFloatinRange (Variables|/Game/Blueprints/Spawners/Waves/PDA_SpawningWave.PDA_SpawningWave_C|GetMinDuration (Variables|Default|GetCurrent%20Wave)) (Variables|/Game/Blueprints/Spawners/Waves/PDA_SpawningWave.PDA_SpawningWave_C|GetMaxDuration (Variables|Default|GetCurrent%20Wave))))
      ;[1 1 1] Retrieve DropChancePerFood
      (Variables|Default|SetDrop%20Chance%20Per%20Food (Variables|/Game/Blueprints/Spawners/Waves/PDA_SpawningWave.PDA_SpawningWave_C|GetDropChancePerFood (Variables|Default|GetCurrent%20Wave)))
      (CallFunction|SpawnFood))))

(fn GetRandomFood
  (bind _drop_chance_per_food (Variables|Default|GetDrop%20Chance%20Per%20Food))
  (LocalVariables|SetRandomValue (Math|Random|RandomIntegerinRange 0 100))
  (bind _keys (Utilities|Map|Keys _drop_chance_per_food))
  (LocalVariables|SetFoods _keys)
  (bind _values (Utilities|Map|Values _drop_chance_per_food))
  (LocalVariables|SetProbabilities _values)
  (bind (_array_element _array_index) (Utilities|Array|ForEachLoopwithBreak (LocalVariables|GetFoods))
    (:LoopBody
      (LocalVariables|SetAssociatedProbability (Utilities|Array|Get(acopy) (LocalVariables|GetProbabilities) _array_index))
      (LocalVariables|SetCumulativeProbability (+ (LocalVariables|GetCumulativeProbability) (LocalVariables|GetAssociatedProbability)))
      (if (>= (LocalVariables|GetCumulativeProbability) (LocalVariables|GetRandomValue))
        (return _array_element)))))

(fn SetWave
  (params (NewIndex :type Integer))
  (Utilities|Time|ClearandInvalidateTimerbyHandle (Variables|Default|GetAutoWaveChangeTH))
  (Variables|Default|SetCurrentWaveIndex (- NewIndex 1))
  (CallFunction|AutoWaveChange))