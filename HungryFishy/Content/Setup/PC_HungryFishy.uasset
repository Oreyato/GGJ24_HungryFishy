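; Player controller for Hungry Fishy that runs the match for several fish sharing one controller.
; BeginPlay sets the shared camera, spawns fish from FishiesDA in a centered row with per-entry looks, and creates the HUD.
; Each fish's Enhanced Input action forwards to a fixed SpawnedFishes index, while StartGame plays the countdown once.
; Tick insertion-sorts fish by score for the scoreboard until one reaches MaxScore, then shows results and lets StartGame reload the map.
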(event Custom|test
  (bind _widgethud (Variables|Default|GetWidgetHUD))
  (bind _sortedarrayactor (Variables|Default|GetSortedArrayActor))
  (bind _sortedarrayactor_2 (Variables|Default|GetSortedArrayActor))
  (bind _wb_finalresult (Variables|/Game/HUD/WB_HUD.WB_HUD_C|GetWB_FinalResult _widgethud))
  (for _array_element (Variables|Fishes|SpawnFishes|GetSpawnedFishes)
    (bind _score (Default|GetScore _array_element))
    (if (>= _score (Variables|Default|GetMaxScore))
      (Variables|Default|SetGameOver true))
    (Variables|Default|SetInsert%20Index (Utilities|Array|Length _sortedarrayactor))
    (bind (_arrayindex _arrayelement) (Utilities|Array|ReverseforEachLoop _sortedarrayactor)
      (:LoopBody
        (bind _score_2 (Default|GetScore _arrayelement))
        (if (< _score _score_2)
          (Variables|Default|SetInsert%20Index _arrayindex)))
      (:Completed
        (Utilities|Array|Insert (Variables|Default|GetSortedArrayActor) _array_element (Variables|Default|GetInsert%20Index)))))
  (if (Variables|Default|GetGameOver)
    (Variables|/Script/UMG.TextBlock|SetText (Variables|/Game/HUD/WB_HUD.WB_HUD_C|GetStartingText _widgethud) (Variables|Default|GetRestartText))
    (Widget|SetVisibility _wb_finalresult "Visible")
    (Widget|SetVisibility (Variables|/Game/HUD/WB_HUD.WB_HUD_C|GetWB_ScoreBoard _widgethud) "Collapsed")
    (Default|ShowFinalResult _wb_finalresult (Variables|Default|GetSortedArrayActor))
    (else
      (Default|UpdateScore (Variables|/Game/HUD/WB_HUD.WB_HUD_C|GetWB_ScoreBoard (Variables|Default|GetWidgetHUD)) _sortedarrayactor_2)
      (Utilities|Array|Clear _sortedarrayactor_2))))

(event Input|EnhancedActionEvents|EnhancedInputActionIA_StartGame
  (params (ActionValue :type Boolean) (ElapsedSeconds :type Float%20%28double-precision%29) (TriggeredSeconds :type Float%20%28double-precision%29) (InputAction :type Input%20Action%20Object%20Reference :default "/Game/Inputs/IA_StartGame.IA_StartGame"))
  (:Triggered
    (if (Variables|Default|GetGameOver)
      (Game|OpenLevel(byObjectReference) "/Game/Maps/LV_MainMap.LV_MainMap"))))

(event Input|EnhancedActionEvents|EnhancedInputActionIA_StartGame
  (params (ActionValue :type Boolean) (ElapsedSeconds :type Float%20%28double-precision%29) (TriggeredSeconds :type Float%20%28double-precision%29) (InputAction :type Input%20Action%20Object%20Reference :default "/Game/Inputs/IA_StartGame.IA_StartGame"))
  (bind _widgethud (Variables|Default|GetWidgetHUD))
  (bind _widgethud_2 (Variables|Default|GetWidgetHUD))
  (:Triggered
    (Utilities|FlowControl|DoOnce false
      (:Completed
        (Widget|SetVisibility (Variables|/Game/HUD/WB_HUD.WB_HUD_C|GetWB_ScoreBoard _widgethud) "Visible")
        (Widget|SetVisibility (Variables|/Game/HUD/WB_HUD.WB_HUD_C|GetStartingText _widgethud) "Hidden")
        (UserInterface|Animation|PlayAnimation _widgethud_2 (Variables|/Game/HUD/WB_HUD.WB_HUD_C|GetCoutdown _widgethud_2) 0.0 1 "Forward" 0.8 false)
        (Audio|PlaySoundatLocation "/Game/Audio/SFX/Countdown.Countdown" "0, 0, 0" "0, 0, 0" 1e+01 1.0 0.0 0 0 0 0)))))

(event Input|EnhancedActionEvents|EnhancedInputActionIA_Fish_Pair
  (params (ActionValue :type Boolean) (ElapsedSeconds :type Float%20%28double-precision%29) (TriggeredSeconds :type Float%20%28double-precision%29) (InputAction :type Input%20Action%20Object%20Reference :default "/Game/Inputs/IA_Fish_Pair.IA_Fish_Pair"))
  (bind _spawnedfishes (Variables|Fishes|SpawnFishes|GetSpawnedFishes))
  (bind _output (Utilities|Array|Get(acopy) _spawnedfishes 3))
  ;[1 1 1] INPUTS
  (:Triggered
    (Default|Triggered _output TriggeredSeconds))
  (:Started
    (Default|Started _output))
  (:Canceled
    (Default|CanceledCompleted _output :!label _label))
  (:Completed
    (goto _label)))

(event Input|EnhancedActionEvents|EnhancedInputActionIA_Fish_Punk
  (params (ActionValue :type Boolean) (ElapsedSeconds :type Float%20%28double-precision%29) (TriggeredSeconds :type Float%20%28double-precision%29) (InputAction :type Input%20Action%20Object%20Reference :default "/Game/Inputs/IA_Fish_Punk.IA_Fish_Punk"))
  (bind _spawnedfishes (Variables|Fishes|SpawnFishes|GetSpawnedFishes))
  (bind _output (Utilities|Array|Get(acopy) _spawnedfishes 4))
  ;[1 1 1] INPUTS
  (:Triggered
    (Default|Triggered _output TriggeredSeconds))
  (:Started
    (Default|Started _output))
  (:Canceled
    (Default|CanceledCompleted _output :!label _label))
  (:Completed
    (goto _label)))

(event Input|EnhancedActionEvents|EnhancedInputActionIA_Fish_Train
  (params (ActionValue :type Boolean) (ElapsedSeconds :type Float%20%28double-precision%29) (TriggeredSeconds :type Float%20%28double-precision%29) (InputAction :type Input%20Action%20Object%20Reference :default "/Game/Inputs/IA_Fish_Train.IA_Fish_Train"))
  (bind _spawnedfishes (Variables|Fishes|SpawnFishes|GetSpawnedFishes))
  (bind _output (Utilities|Array|Get(acopy) _spawnedfishes 5))
  ;[1 1 1] INPUTS
  (:Triggered
    (Default|Triggered _output TriggeredSeconds))
  (:Started
    (Default|Started _output))
  (:Canceled
    (Default|CanceledCompleted _output :!label _label))
  (:Completed
    (goto _label)))

(event Input|EnhancedActionEvents|EnhancedInputActionIA_Fish_Bee
  (params (ActionValue :type Boolean) (ElapsedSeconds :type Float%20%28double-precision%29) (TriggeredSeconds :type Float%20%28double-precision%29) (InputAction :type Input%20Action%20Object%20Reference :default "/Game/Inputs/IA_Fish_Bee.IA_Fish_Bee"))
  (bind _spawnedfishes (Variables|Fishes|SpawnFishes|GetSpawnedFishes))
  (bind _output (Utilities|Array|Get(acopy) _spawnedfishes))
  ;[1 1 1] INPUTS
  (:Triggered
    (Default|Triggered _output TriggeredSeconds))
  (:Started
    (Default|Started _output))
  (:Canceled
    (Default|CanceledCompleted _output :!label _label))
  (:Completed
    (goto _label)))

(event Input|EnhancedActionEvents|EnhancedInputActionIA_Fish_Car
  (params (ActionValue :type Boolean) (ElapsedSeconds :type Float%20%28double-precision%29) (TriggeredSeconds :type Float%20%28double-precision%29) (InputAction :type Input%20Action%20Object%20Reference :default "/Game/Inputs/IA_Fish_Car.IA_Fish_Car"))
  (bind _spawnedfishes (Variables|Fishes|SpawnFishes|GetSpawnedFishes))
  (bind _output (Utilities|Array|Get(acopy) _spawnedfishes 1))
  ;[1 1 1] INPUTS
  (:Triggered
    (Default|Triggered _output TriggeredSeconds))
  (:Started
    (Default|Started _output))
  (:Canceled
    (Default|CanceledCompleted _output :!label _label))
  (:Completed
    (goto _label)))

(event Input|EnhancedActionEvents|EnhancedInputActionIA_Fish_Cowboy
  (params (ActionValue :type Boolean) (ElapsedSeconds :type Float%20%28double-precision%29) (TriggeredSeconds :type Float%20%28double-precision%29) (InputAction :type Input%20Action%20Object%20Reference :default "/Game/Inputs/IA_Fish_Cowboy.IA_Fish_Cowboy"))
  (bind _spawnedfishes (Variables|Fishes|SpawnFishes|GetSpawnedFishes))
  (bind _output (Utilities|Array|Get(acopy) _spawnedfishes 2))
  ;[1 1 1] INPUTS
  (:Triggered
    (Default|Triggered _output TriggeredSeconds))
  (:Started
    (Default|Started _output))
  (:Canceled
    (Default|CanceledCompleted _output :!label _label))
  (:Completed
    (goto _label)))

(event EventBeginPlay
  (bind _returnvalue (Actor|GetActorOfClass "/Game/Setup/BP_NewCamera.BP_NewCamera_C"))
  (bind _output_get (Variables|Default|SetMainCamera _returnvalue))
  (Game|Player|SetViewTargetwithBlend _output_get 0.0 "VTBlend_Linear" 0.0 false)
  (CallFunction|TrySetSpawnCenterLocation)
  (CallFunction|SetInitialSpawnParameters)
  (bind (_array_element _array_index) (Utilities|Array|ForEachLoopwithBreak (Variables|Fishes|GetFishiesDA))
    (:LoopBody
      (bind _output_get_2 (Variables|Default|SetArray%20Index _array_index))
      (bind _transformlocation (CallFunction|SetFishSpawnLocationBasedonIndex _output_get_2))
      (bind _returnvalue_2 (Game|SpawnActorfromClass "/Game/Blueprints/Fishy/BP_FishNew.BP_FishNew_C" (Math|Transform|MakeTransform _transformlocation "0, 0, 0" "1.000000,1.000000,1.000000") "AdjustIfPossibleButAlwaysSpawn" "MultiplyWithRoot" 0 0))
      (Components|StaticMesh|SetStaticMesh (Variables|/Game/Blueprints/Fishy/BP_FishNew.BP_FishNew_C|GetBody _returnvalue_2) (Variables|/Game/Blueprints/Fishy/Data/PDA_Fish.PDA_Fish_C|GetBodyMesh _array_element))
      (Default|SetCustomTailColor _returnvalue_2 (Variables|/Game/Blueprints/Fishy/Data/PDA_Fish.PDA_Fish_C|GetColor _array_element))
      (Variables|/Game/Blueprints/Fishy/BP_FishNew.BP_FishNew_C|SetFishicon _returnvalue_2 (Variables|/Game/Blueprints/Fishy/Data/PDA_Fish.PDA_Fish_C|GetIconUI _array_element))
      (Rendering|Components|Sprite|SetSprite (Variables|/Game/Blueprints/Fishy/BP_FishNew.BP_FishNew_C|GetInputIcon _returnvalue_2) (Variables|/Game/Blueprints/Fishy/Data/PDA_Fish.PDA_Fish_C|GetInputIcon _array_element))
      (Utilities|Array|Add (Variables|Fishes|SpawnFishes|GetSpawnedFishes) _returnvalue_2))
    (:Completed
      (bind _returnvalue_3 (UserInterface|CreateWidget "/Game/HUD/WB_HUD.WB_HUD_C"))
      (bind _output_get_3 (Variables|Default|SetWidgetHUD _returnvalue_3))
      (UserInterface|Viewport|AddtoViewport _output_get_3 0))))

(event EventTick
  (params (DeltaSeconds :type Float%20%28single-precision%29))
  (bind _widgethud (Variables|Default|GetWidgetHUD))
  (bind _sortedarrayactor (Variables|Default|GetSortedArrayActor))
  (bind _sortedarrayactor_2 (Variables|Default|GetSortedArrayActor))
  (bind _wb_finalresult (Variables|/Game/HUD/WB_HUD.WB_HUD_C|GetWB_FinalResult _widgethud))
  (if (not (Variables|Default|GetGameOver))
    (for _array_element (Variables|Fishes|SpawnFishes|GetSpawnedFishes)
      (bind _score (Default|GetScore _array_element))
      (if (>= _score (Variables|Default|GetMaxScore))
        (Variables|Default|SetGameOver true))
      (Variables|Default|SetInsert%20Index (Utilities|Array|Length _sortedarrayactor))
      (bind (_arrayindex _arrayelement) (Utilities|Array|ReverseforEachLoop _sortedarrayactor)
        (:LoopBody
          (bind _score_2 (Default|GetScore _arrayelement))
          (if (< _score _score_2)
            (Variables|Default|SetInsert%20Index _arrayindex)))
        (:Completed
          (Utilities|Array|Insert (Variables|Default|GetSortedArrayActor) _array_element (Variables|Default|GetInsert%20Index)))))
    (if (Variables|Default|GetGameOver)
      (Variables|/Script/UMG.TextBlock|SetText (Variables|/Game/HUD/WB_HUD.WB_HUD_C|GetStartingText _widgethud) (Variables|Default|GetRestartText))
      (Widget|SetVisibility _wb_finalresult "Visible")
      (Widget|SetVisibility (Variables|/Game/HUD/WB_HUD.WB_HUD_C|GetWB_ScoreBoard _widgethud) "Collapsed")
      (Default|ShowFinalResult _wb_finalresult (Variables|Default|GetSortedArrayActor))
      (else
        (Default|UpdateScore (Variables|/Game/HUD/WB_HUD.WB_HUD_C|GetWB_ScoreBoard (Variables|Default|GetWidgetHUD)) _sortedarrayactor_2)
        (Utilities|Array|Clear _sortedarrayactor_2)))))

(fn ConstructionScript)

(fn TrySetSpawnCenterLocation
  (bind _returnvalue (Actor|GetActorOfClass "/Game/Setup/BP_SpawnCenterLocation.BP_SpawnCenterLocation_C"))
  (Utilities|IsValid _returnvalue
    (:Is%20Valid
      (Variables|Fishes|SpawnFishes|SetSpawnCenterLocation (Transformation|GetActorLocation _returnvalue))
      (return))
    (:Is%20Not%20Valid
      (Development|PrintString "An actor of type BP_SpawnCenterLocation is missing")
      (return))))

(fn SetFishSpawnLocationBasedonIndex
  (params (Index :type Integer))
  (bind _output_get (Variables|Fishes|SpawnFishes|SetSpawn%20Transform%20Location (+ (Variables|Fishes|SpawnFishes|GetSpawnCenterLocation) (Math|Vector|MakeVector 0.0 (+ (Variables|Fishes|SpawnFishes|GetLeftMostOffset) (* (Variables|Fishes|SpawnFishes|GetTotalDistance) (/ Index (Utilities|Array|Length (Variables|Fishes|GetFishiesDA))))) 0.0))))
  (return _output_get))

(fn SetInitialSpawnParameters
  (Variables|Fishes|SpawnFishes|SetTotalDistance (* (Variables|Fishes|SpawnFishes|GetDistanceBetweenFishes) (Utilities|Array|Length (Variables|Fishes|GetFishiesDA))))
  (Variables|Fishes|SpawnFishes|SetLeftMostOffset (* (/ (Variables|Fishes|SpawnFishes|GetTotalDistance) 2.0) -1.0)))